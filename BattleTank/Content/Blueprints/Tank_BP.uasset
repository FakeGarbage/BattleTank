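; Tank pawn Blueprint that wires player input to aiming, firing and tracked movement components.
; Construction script and BeginPlay both hand the barrel and turret to TankAiming and the two tracks to TankMovement.
; Axis input sends move and turn intents to TankMovement and rotates the Gimbal and SpringArm for camera aim, while Fire calls TankAiming.
; BeginPlay also passes the tank to its Healthbar widget.
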(event `self.ReceiveBeginPlay`
  (`TankAimingComponent.Initialize` (`self.TankAiming`) (`self.TankBarrel`) (`self.TankTurret`))
  (`TankMovementComponent.Initialize` (`self.TankMovement`) (`self.LeftTrack`) (`self.RightTrack`))
  (`self.InitializeHealthBarWidget`))

(event `InputAxis|AimVertical`
  (params (AxisValue :type "Float (single-precision)"))
  ;[1 1 1] firing/aiming setup
  (`SceneComponent.K2_AddLocalRotation` (`self.SpringArm`) (`KismetMathLibrary.MakeRotator` 0.0 AxisValue) false false))

(event `InputAction|Fire`
  (params (Key :type "Key Structure"))
  ;[1 1 1] firing/aiming setup
  (:`Pressed`
    (`TankAimingComponent.FireTankProjectile` (`self.TankAiming`))))

(event `InputAxis|Forward`
  (params (AxisValue :type "Float (single-precision)"))
  ;[1 1 1] Movement Input Setup
  (`TankMovementComponent.IntendMoveForward` (`self.TankMovement`) AxisValue))

(event `InputAxis|TurnRight`
  (params (AxisValue :type "Float (single-precision)"))
  ;[1 1 1] Movement Input Setup
  (`TankMovementComponent.IntendTurnRight` (`self.TankMovement`) AxisValue))

(event `InputAxis|AimHorizontal`
  (params (AxisValue :type "Float (single-precision)"))
  ;[1 1 1] firing/aiming setup
  (`SceneComponent.K2_AddLocalRotation` (`self.Gimbal`) (`KismetMathLibrary.MakeRotator` 0.0 0.0 AxisValue) false false))

(event `InputAxis|TurnLeft`
  (params (AxisValue :type "Float (single-precision)"))
  ;[1 1 1] Movement Input Setup
  (`TankMovementComponent.IntendTurnLeft` (`self.TankMovement`) AxisValue))

(fn `InitializeHealthBarWidget`
  (bind _ashealthbar (cast `/Game/UI/Healthbar` (`WidgetComponent.GetUserWidgetObject` (`self.Widget`))))
  (set `/Game/UI/Healthbar.Tank` self _ashealthbar)
  (return))

(fn `UserConstructionScript`
  (`TankAimingComponent.Initialize` (`self.TankAiming`) (`self.TankBarrel`) (`self.TankTurret`))
  (`TankMovementComponent.Initialize` (`self.TankMovement`) (`self.LeftTrack`) (`self.RightTrack`)))